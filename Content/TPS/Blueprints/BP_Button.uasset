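; BP_Button is an interactable button that positions the interacting player and plays a press montage on their character.
; On the interactable component's Interacted event, it disables TPS character controls and plays the montage, re-enabling them on completion, interruption or either montage notify.
; It then snaps the player's control rotation and teleports the pawn to a Capsule child actor's transform, lining the character up with the button.
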(event Interacted(BP_InteractableComponent)
  (params (Pawn :type Pawn%20Object%20Reference) (Player :type Player%20Controller%20Object%20Reference))
  (bind _capsule (Variables|Default|GetCapsule))
  (bind _childactor (Variables|/Script/Engine.ChildActorComponent|GetChildActor _capsule))
  (bind _returnvalue (Transformation|GetActorRotation _childactor))
  (Utilities|FlowControl|Sequence
    (:then_0
      (bind _asbp_tpscharacter (Utilities|Casting|CastToBP_TPSCharacter Pawn))
      (Default|SetControlsDisabled _asbp_tpscharacter true)
      (Animation|Montage|PlayMontage (Variables|/Script/Engine.Character|GetMesh _asbp_tpscharacter) (Variables|Default|GetMontage%20to%20Play)
        (:OnCompleted
          _)
        (:OnInterrupted
          _)
        (:OnNotifyBegin
          _)
        (:OnNotifyEnd
          _))
      (Default|SetControlsDisabled _asbp_tpscharacter false))
    (:then_1
      (Pawn|SetControlRotation Player _returnvalue)
      (Transformation|Teleport Pawn (Transformation|GetActorLocation _childactor) _returnvalue))))

(fn ConstructionScript)