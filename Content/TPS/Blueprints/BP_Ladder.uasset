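; BP_Ladder is a ladder actor whose height is set by a Size value, clamped to at least one.
; Its construction script stretches and raises a Box component to match Size, keeping its base at the relative origin.
; It then rebuilds the ladder from instanced static mesh segments, each offset by a multiple of StepSize.
; The event graph holds only disabled placeholder events, so this Blueprint defines no climbing logic.
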(event EventBeginPlay)

(event Collision|EventActorBeginOverlap
  (params (OtherActor :type Actor%20Object%20Reference)))

(event EventTick
  (params (DeltaSeconds :type Float%20%28single-precision%29)))

(fn ConstructionScript
  (bind _instancedstaticmesh (Variables|Default|GetInstancedStaticMesh))
  (bind _box (Variables|Default|GetBox))
  (bind _output_get (Variables|Default|SetSize (Math|Integer|Max(Integer) 1 (stale _output_get))))
  (Components|Box|SetBoxExtent _box (Math|Vector|MakeVector 5e+01 5e+01 (* (Variables|Default|GetSize) 1e+02)) false)
  (Transformation|SetRelativeLocation _box (Math|Vector|MakeVector 0.0 0.0 (* (Variables|Default|GetSize) 1e+02)) false false)
  (Components|InstancedStaticMesh|ClearInstances _instancedstaticmesh)
  (for _index (range 0 (- (Variables|Default|GetSize) 1))
    (Components|InstancedStaticMesh|AddInstance _instancedstaticmesh (Math|Transform|MakeTransform (* (Variables|Default|GetStepSize) _index)) false)))