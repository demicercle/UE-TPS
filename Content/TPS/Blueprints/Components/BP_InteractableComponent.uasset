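; BP_InteractableComponent is a component that makes its owning actor interactable by a player.
; Interact broadcasts the Interacted event dispatcher with the pawn and player, leaving the response to bound listeners.
; DrawDebug outlines the owner's colliding bounds with a box at the actor's rotation, draws a short line up from the bounds center, and prints InteractionText just above it.
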(fn Interact
  (params (Pawn :type Pawn%20Object%20Reference) (Player :type Player%20Controller%20Object%20Reference))
  (Default|CallInteracted Pawn Player))

(fn DrawDebug
  (bind _returnvalue (Components|GetOwner))
  (bind (_origin _boxextent) (Collision|GetActorBounds _returnvalue true false))
  (bind _returnvalue_2 (+ _origin (Math|Vector|MakeVector 0.0 0.0 32.0)))
  (Rendering|Debug|DrawDebugBox _origin _boxextent "(R=1.000000,G=1.000000,B=1.000000,A=1.000000)" (Transformation|GetActorRotation _returnvalue) 0.0 1.0)
  (Rendering|Debug|DrawDebugLine _origin _returnvalue_2 "(R=1.000000,G=1.000000,B=1.000000,A=1.000000)" 0.0 1.0)
  (Rendering|Debug|DrawDebugString (+ _returnvalue_2 (Math|Vector|MakeVector 0.0 0.0 8.0)) (Utilities|String|ToString(Text) (Variables|Default|GetInteractionText)) 0 "(R=1.000000,G=1.000000,B=1.000000,A=1.000000)"))