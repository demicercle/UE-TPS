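; Inventory component that tracks carried items as a map of item IDs to stack counts.
; AddItem and RemoveItem adjust the counts, dropping an entry when it empties, and FindItem returns data for held items.
; GetItemData looks IDs up in an item data table, falling back to the first valid row when the ID is missing.
; With Debug enabled, Tick prints item names and counts on screen.
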(event EventTick
  (params (DeltaSeconds :type Float%20%28single-precision%29))
  (if (Variables|Default|GetDebug)
    (CallFunction|PrintInventory)))

(fn AddItem
  (params (NewItem :type Name))
  (bind _slots (Variables|Default|GetSlots))
  (bind (_value _returnvalue) (Utilities|Map|Find _slots NewItem))
  (Utilities|Map|Keys _slots)
  (if _returnvalue
    (Math|Integer|IncrementInt _value)
    (else
      (Utilities|Map|Add _slots NewItem 1))))

(fn PrintInventory
  (bind _slots (Variables|Default|GetSlots))
  (bind _keys (Utilities|Map|Keys _slots))
  (for _array_element _keys
    (bind (_success _item) (CallFunction|GetItemData _array_element))
    (Development|PrintString (Utilities|String|SelectString (Utilities|String|Append (Utilities|String|ToString(Text) (.DisplayedName (Utilities|Struct|BreakS_InventoryItem _item))) " (" (Utilities|String|ToString(Integer) (.Value (Utilities|Map|Find _slots _array_element))) ")") (Utilities|String|Append "Invalid Item ID: " (Utilities|String|ToString(Name) _array_element)) _success) true false "(R=1.000000,G=1.000000,B=1.000000,A=1.000000)" 0.0)))

(fn RemoveItem
  (params (ID :type Name))
  (bind _slots (Variables|Default|GetSlots))
  (bind (_value _returnvalue) (Utilities|Map|Find _slots ID))
  (if _returnvalue
    (bind _result (Math|Integer|DecrementInt _value)
      (:%20%20
        (if (<= _result 0)
          (Utilities|Map|Remove _slots ID)
          (return true))))
    (else
      (return false))))

(fn FindItem
  (params (ID :type Name))
  (if (.ReturnValue (Utilities|Map|Find (Variables|Default|GetSlots) ID))
    (bind (_success _item) (CallFunction|GetItemData ID))
    (return _success _item)
    (else
      (return false ""))))

(fn GetItemData
  (params (ID :type Name))
  (bind _itemdatatable (Variables|Default|GetItemDataTable))
  (bind _returnvalue (Utilities|GetDataTableRow _itemdatatable ID)
    (:then
      (return true _returnvalue))
    (:RowNotFound
      (bind _outrownames (DataTable|GetDataTableRowNames _itemdatatable))
      (for _array_element _outrownames
        (bind _returnvalue_2 (Utilities|GetDataTableRow _itemdatatable _array_element)
          (:then
            (return true _returnvalue_2))))
      (return false ""))))