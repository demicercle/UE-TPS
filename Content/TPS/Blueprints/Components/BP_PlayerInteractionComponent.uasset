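; Player component that finds interactable actors in front of the owning pawn and triggers them on the IA_Interact input.
; Each tick, a sphere overlap takes the first actor with BP_InteractableComponent that passes a facing dot-product test, unless interaction is disabled.
; W_Interaction is projected onto that actor's bounds center, with a debug box drawn regardless of the Debug flag, which only shows the search radius.
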(event Input|EnhancedActionEvents|EnhancedInputActionIA_Interact
  (params (ActionValue :type Boolean) (ElapsedSeconds :type Float%20%28double-precision%29) (TriggeredSeconds :type Float%20%28double-precision%29) (InputAction :type Input%20Action%20Object%20Reference :default "/Game/TPS/Input/Actions/IA_Interact.IA_Interact"))
  (bind _interactable (Variables|Default|GetInteractable))
  (:Started
    (Utilities|IsValid _interactable
      (:Is%20Valid
        (Default|Interact _interactable (Variables|Default|GetOwningPawn) (Variables|Default|GetOwningPlayer))))))

(event EventTick
  (params (DeltaSeconds :type Float%20%28single-precision%29))
  (bind _widget (Variables|Default|GetWidget))
  (Utilities|FlowControl|Sequence
    (:then_0
      (bind (_success _interactable _hitactor) (CallFunction|FindInteractable))
      (bind _output_get (Variables|Default|SetInteractable _interactable))
      (Utilities|IsValid _output_get
        (:Is%20Valid
          (UserInterface|Viewport|AddtoViewport _widget 0)
          (Class|UserWidget|SetPositioninViewport _widget (.ScreenPosition (Class|GameplayStatics|ProjectWorldtoScreen (Variables|Default|GetOwningPlayer) (.Origin (Collision|GetActorBounds _hitactor true false)) false)) true)
          (Rendering|Debug|DrawDebugBox (.Origin (Collision|GetActorBounds _hitactor true false)) (.BoxExtent (Collision|GetActorBounds _hitactor true false)) "(R=1.000000,G=1.000000,B=1.000000,A=1.000000)" (Transformation|GetActorRotation _hitactor) 0.0 1.0))
        (:Is%20Not%20Valid
          (Widget|RemovefromParent _widget))))
    (:then_1
      (if (Variables|Default|GetDebug)
        (Rendering|Debug|DrawDebugSphere (Transformation|GetActorLocation (Components|GetOwner)) (Variables|Default|GetInteractRadius) 12 "(R=1.000000,G=1.000000,B=1.000000,A=1.000000)" 0.0 1.0)))))

(event EventBeginPlay
  (bind _aspawn (Utilities|Casting|CastToPawn (Components|GetOwner)))
  (Variables|Default|SetOwningPawn _aspawn)
  (bind _asplayer_controller (Utilities|Casting|CastToPlayerController (Pawn|GetController _aspawn)))
  (bind _output_get (Variables|Default|SetOwningPlayer _asplayer_controller))
  (bind _returnvalue (UserInterface|CreateWidget "/Game/TPS/Widgets/W_Interaction.W_Interaction_C" _output_get))
  (Variables|Default|SetWidget _returnvalue))

(fn FindInteractable
  (bind _returnvalue (Components|GetOwner))
  (bind _returnvalue_2 (Transformation|GetActorLocation _returnvalue))
  (if (Variables|Default|GetDisableInteraction)
    (return false 0 0)
    (else
      (bind _outactors (Collision|SphereOverlapActors _returnvalue_2 (Variables|Default|GetInteractRadius) (Utilities|Array|MakeArray "ObjectTypeQuery1" "ObjectTypeQuery2" "ObjectTypeQuery3" "ObjectTypeQuery4" "ObjectTypeQuery5" "ObjectTypeQuery6") "/Script/Engine.Actor" (Utilities|Array|MakeArray _returnvalue)))
      (for _array_element _outactors
        (Utilities|IsValid (Actor|GetComponentbyClass _array_element "/Game/TPS/Blueprints/Components/BP_InteractableComponent.BP_InteractableComponent_C")
          (:Is%20Valid
            (if (>= (Math|Vector|DotProduct (Transformation|GetActorForwardVector _returnvalue) (Math|Vector|GetForwardVector (Math|Rotator|FindLookatRotation _returnvalue_2 (Transformation|GetActorLocation _array_element)))) (Variables|Default|GetMinDotProductToInteract))
              (return true (Actor|GetComponentbyClass _array_element "/Game/TPS/Blueprints/Components/BP_InteractableComponent.BP_InteractableComponent_C") _array_element)))))
      (return false 0 0))))